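; Main terminal usable that runs the timed data-transfer quest objective, offering its prompt and one-time start only during the TransferData stage.
; Once started, Tick accumulates progress, which pauses while any sub-terminal is overheating.
; Looping timers drive the hazards: random sub-terminal overheats and android spawns from linked spawners, capped by a live count that death events decrement.
; On completion it clears both timers and sets the gamemode's stage to DataTransferred.
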(event `self.ReceiveTick`
  (params (DeltaSeconds :type "Float (single-precision)"))
  (bind _asndgamemode_bp (cast `/Game/Blueprints/NDGamemode_BP` (`GameplayStatics.GetGameMode`)))
  (bind _returnvalue (`EscapeGameModeBase.GetQuestStage` _asndgamemode_bp))
  (if (`|EnumEquality` _returnvalue "TransferData")
    (set `self.Prompt` "Transfer Data")
    (else
      (set `self.Prompt` "")))
  (if (`self.bIsProgressing`)
    (`self.UpdateProgress`)))

(event `self.Use`
  (bind _asndgamemode_bp (cast `/Game/Blueprints/NDGamemode_BP` (`GameplayStatics.GetGameMode`)))
  (bind _returnvalue (`EscapeGameModeBase.GetQuestStage` _asndgamemode_bp))
  (if (`|EnumEquality` _returnvalue "TransferData")
    (`/Engine/EditorBlueprintResources/StandardMacros.DoOnce` false
      (:`Completed`
        (`self.StartProgress`)))))

(event `OnSpawnedAndroidDeath`
  (`/Engine/EditorBlueprintResources/StandardMacros.DecrementInt` (`self.AndroidCount`)))

(fn `EndProgress`
  (`KismetSystemLibrary.K2_ClearAndInvalidateTimerHandle` (`self.AndroidTimerHandle`))
  (`KismetSystemLibrary.K2_ClearAndInvalidateTimerHandle` (`self.TerminalTimerHandle`))
  (bind _asndgamemode_bp (cast `/Game/Blueprints/NDGamemode_BP` (`GameplayStatics.GetGameMode`)))
  (`EscapeGameModeBase.SetQuestStage` _asndgamemode_bp "DataTransferred"))

(fn `OverheatSubTerminal`
  (bind _subterminals (`self.SubTerminals`))
  (`/Game/Blueprints/Usable_SubTerminal_BP.Overheat` (`KismetArrayLibrary.Array_Get` _subterminals (`KismetMathLibrary.RandomIntegerInRange` 0 (- (`KismetArrayLibrary.Array_Length` _subterminals) 1)))))

(fn `SpawnAndroids`
  (for _array_element (`self.AndroidSpawners`)
    (if (<= (`self.AndroidCount`) (`self.TotalAndroidLimit`))
      (bind _androids (`/Game/Blueprints/AndroidSpawner.SpawnAndroid` _array_element 1))
      (for _array_element_2 _androids
        (add `AndroidCharacter.OnDeath` _array_element_2 (`|CreateDelegate` :!event `OnSpawnedAndroidDeath`)))
      (`/Engine/EditorBlueprintResources/StandardMacros.IncrementInt` (`self.AndroidCount`))
      (else
        (return))))
  (return))

(fn `StartProgress`
  (set `self.bIsProgressing` true)
  (bind _returnvalue (`KismetSystemLibrary.K2_SetTimerDelegate` (`|CreateDelegate` :!event `OverheatSubTerminal`) 15.0 true))
  (set `self.TerminalTimerHandle` _returnvalue)
  (bind _returnvalue_2 (`KismetSystemLibrary.K2_SetTimerDelegate` (`|CreateDelegate` :!event `SpawnAndroids`) 12.0 true))
  (set `self.AndroidTimerHandle` _returnvalue_2)
  (return))

(fn `UpdateProgress`
  (`|ExecutionSequence`
    (:`then_0`
      (for _array_element (`self.SubTerminals`)
        (if (not (not (`/Game/Blueprints/Usable_SubTerminal_BP.bIsOverheating` _array_element)))
          (return)))
      (bind _output_get (set `self.Progress` (+ (`GameplayStatics.GetWorldDeltaSeconds`) (`self.Progress`))))
      (`KismetSystemLibrary.PrintString` (`KismetStringLibrary.Conv_DoubleToString` _output_get) true true (struct :`G` 0.66 :`B` 1.0 :`A` 1.0) 0.0))
    (:`then_1`
      (if (>= (`self.Progress`) (`self.TotalProgressTime`))
        (set `self.bIsProgressing` false)
        (`self.EndProgress`))
      (return))))

(fn `UserConstructionScript`
  (`parent.UserConstructionScript`))