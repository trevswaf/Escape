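; A usable door Blueprint that either slides open or signals that it is locked.
; On Use, a locked door plays its audio component unless it is already playing, while an unlocked door fires DoorOpenEvent.
; That event plays the DoorOpen timeline, which moves the mesh along its relative X axis.
; The construction script runs the parent's script, then assigns the Speech sound to the audio component.
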(event `self.Use`
  (bind _audio (`self.Audio`))
  (if (`self.bLocked`)
    ;[1 1 1] If door is locked play audio notifier, assuming it isn't currently playing
    (if (not (`AudioComponent.IsPlaying` _audio))
      (`AudioComponent.Play` _audio 0.0))
    (else
      ;[1 1 1] Prototype implementation of opening door by destroying it
      (`self.DoorOpenEvent`))))

(event `DoorOpenEvent`
  (bind (_direction _x_value) (`Timeline|DoorOpen`)
    (:`Update`
      (`SceneComponent.K2_SetRelativeLocation` (`self.Mesh`) (`KismetMathLibrary.MakeVector` _x_value) false false))))

(fn `UserConstructionScript`
  (`parent.UserConstructionScript`)
  (`AudioComponent.SetSound` (`self.Audio`) "/Game/Audio/speech.speech"))