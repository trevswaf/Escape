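; Usable exit terminal that reacts to the current quest stage held by the NDGamemode_BP game mode.
; Tick polls the stage and shows a "Use Terminal" prompt only at Grab Key, Power Turned on and Data Transferred.
; Using it at Grab Key plays a one-time voice line; at Data Transferred it plays the monologue level sequence.
; Power Turned on shows the prompt but has no Use response here.
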(event `self.ReceiveTick`
  (params (DeltaSeconds :type "Float (single-precision)"))
  (bind _returnvalue (`EscapeGameModeBase.GetQuestStage` (`self.GameMode`)))
  (switch `EQuestStage` _returnvalue
    (:`Intro`
      (set `self.Prompt` "" :!label _label))
    (:`GrabGun`
      (goto _label))
    (:`DoorLocked`
      (goto _label))
    (:`AndroidEncounter`
      (goto _label))
    (:`GrabKey`
      (set `self.Prompt` "Use Terminal" :!label _label_2))
    (:`TurnOnPower`
      (goto _label))
    (:`PowerTurnedOn`
      (goto _label_2))
    (:`TransferData`
      (goto _label))
    (:`DataTransferred`
      (goto _label_2))))

(event `self.ReceiveBeginPlay`
  (bind _asndgamemode_bp (cast `/Game/Blueprints/NDGamemode_BP` (`GameplayStatics.GetGameMode`)))
  (set `self.GameMode` _asndgamemode_bp))

(event `self.Use`
  (bind _returnvalue (`EscapeGameModeBase.GetQuestStage` (`self.GameMode`)))
  (switch `EQuestStage` _returnvalue
    (:`GrabKey`
      (`/Engine/EditorBlueprintResources/StandardMacros.DoOnce` false
        (:`Completed`
          (`/Game/Blueprints/Voice.VoicePlay` (`/Game/Blueprints/NDGamemode_BP.Voice` (`self.GameMode`)) 3)
          (set `self.Prompt` ""))))
    (:`DataTransferred`
      (bind _returnvalue_2 (`LevelSequencePlayer.CreateLevelSequencePlayer` self (`self.MonologueSequence`)))
      (`LevelSequencePlayer.Play` _returnvalue_2))))

(fn `UserConstructionScript`
  (`parent.UserConstructionScript`))