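; Game mode Blueprint that sets up the HUD, audio and display when play begins.
; A BeginPlay sequence first adds the PlayerHUD widget to the viewport, spawns an AmbientSound actor playing ServerAmbient, and forces fullscreen through GameUserSettings.
; It then spawns a Voice actor, keeping references to it, the HUD widget and the ambient audio actor.
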(event `self.ReceiveBeginPlay`
  (bind _returnvalue (`KismetMathLibrary.MakeTransform` (0.0 0.0 0.0)))
  (`|ExecutionSequence`
    (:`then_0`
      (bind _returnvalue_2 (`|CreateWidget` "/Game/UI/PlayerHUD.PlayerHUD_C"))
      (bind _output_get (set `self.WidgetReference` _returnvalue_2))
      (`UserWidget.AddToViewport` _output_get 0)
      (bind _returnvalue_3 (`|SpawnActorFromClass` "/Script/Engine.AmbientSound" _returnvalue "Undefined" "OverrideRootScale"))
      (bind _output_get_2 (set `self.AmbientAudio` _returnvalue_3))
      (bind _audiocomponent (`AmbientSound.AudioComponent` _output_get_2))
      (`AudioComponent.SetSound` _audiocomponent "/Game/Audio/ServerAmbient.ServerAmbient")
      (`AudioComponent.Play` _audiocomponent 0.0)
      (bind _returnvalue_4 (`GameUserSettings.GetGameUserSettings`))
      (`GameUserSettings.SetFullscreenMode` _returnvalue_4 "Fullscreen")
      (`GameUserSettings.ApplySettings` _returnvalue_4 true))
    (:`then_1`
      (bind _returnvalue_5 (`|SpawnActorFromClass` "/Game/Blueprints/Voice.Voice_C" _returnvalue "Undefined" "OverrideRootScale"))
      (set `self.Voice` _returnvalue_5))))

(fn `UserConstructionScript`)