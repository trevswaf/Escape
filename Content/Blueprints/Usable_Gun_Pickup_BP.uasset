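; Usable gun pickup that arms the player when used.
; Use reveals the hidden PrototypeGun mesh on the player's FPSCharacter_BP and resets its shoot cooldown.
; It then sets the NDGamemode_BP quest stage to GrabGun and destroys itself.
; A TODO notes that enabling the player's ability to shoot is still pending.
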(event `self.Use`
  ;[1 1 1] Render player weapon mesh. TODO set can shoot to true.
  (bind _asfpscharacter_bp (cast `/Game/Blueprints/FPSCharacter_BP` (`GameplayStatics.GetPlayerCharacter` 0)))
  (`SceneComponent.SetHiddenInGame` (`/Game/Blueprints/FPSCharacter_BP.PrototypeGun` _asfpscharacter_bp) false false)
  (`FPSCharacter.ResetShootCooldown` _asfpscharacter_bp)
  (bind _asndgamemode_bp (cast `/Game/Blueprints/NDGamemode_BP` (`GameplayStatics.GetGameMode`)))
  (`EscapeGameModeBase.SetQuestStage` _asndgamemode_bp "GrabGun")
  (`self.K2_DestroyActor`))

(fn `UserConstructionScript`
  (`parent.UserConstructionScript`))