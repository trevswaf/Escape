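; First-person player character that handles charge-gun feedback, damage, death, respawn and pausing.
; Binds charge, shoot, damage and sprint events to drive the gun's dynamic glow material, AnimBP, audio, particles, camera shake, post-processing and FOV.
; Timelines animate gun bob, glow color and camera effects.
; Game mode supplies HUD, voice pausing and quest stage, which decides between respawn and Credits; playing level sequences block pausing.
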(event `self.ReceiveBeginPlay`
  (bind _asgun_anim_bp (cast `/Game/Models/Weapon/Gun_AnimBP` (`SkeletalMeshComponent.GetAnimInstance` (`self.Gun`))))
  (set `self.AnimBP` _asgun_anim_bp)
  (add `self.OnDamaged` (`|CreateDelegate` :!event `DamageEffects`))
  (bind (_direction _offset) (`Timeline|GunIdle` :!via `PlayFromStart` :!label _label)
    (:`Update`
      (`SceneComponent.K2_SetRelativeLocation` (`self.Gun`) (+ (`KismetMathLibrary.MakeVector` 0.0 0.0 _offset) (`self.BeginingGunLocation`)) false false))
    (:`Finished`
      (`self.Finished`))))

(event `Finished`
  (goto _label :!via `PlayFromStart`))

(event `Key|L`
  (params (Key :type "Key Structure" :default "AnyKey"))
  (:`Pressed`
    (`KismetSystemLibrary.ExecuteConsoleCommand` "HighResShot 1" (`GameplayStatics.GetPlayerController` 0))))

(event `SetColorBlue`
  (params (RechargeTime :type "Float (double-precision)"))
  (`|ExecutionSequence`
    (:`then_0`
      (bind (_direction _colortrack) (`Timeline|Gun_Color_Lerp` :`NewTime` (- 0.5 RechargeTime) :!via `SetNewTime` :!label _label_2)
        (:`Update`
          (`MaterialInstanceDynamic.SetVectorParameterValue` (`self.GunGlowMaterial`) "Emissive Color" _colortrack))))
    (:`then_1`
      (goto _label_2))))

(event `InputAction|Objective`
  (params (Key :type "Key Structure" :default "AnyKey"))
  (:`Pressed`
    (bind _asndgamemode_bp (cast `/Game/Blueprints/NDGamemode_BP` (`GameplayStatics.GetGameMode`)))
    (`/Game/UI/PlayerHUD.PlayObjectiveAnimation` (`/Game/Blueprints/NDGamemode_BP.WidgetReference` _asndgamemode_bp))))

(event `OnSprintEvent`
  (params (bIsSprinting :type Boolean))
  (if bIsSprinting
    (bind (_direction _fov) (`Timeline|CameraFOV` :!label _label_3)
      (:`Update`
        (`CameraComponent.SetFieldOfView` (`self.FirstPersonCamera`) _fov)))
    (else
      (goto _label_3 :!via `Reverse`))))

(event `UpdatePostProcessing`
  (bind (_direction _vignetteintensity _scale) (`Timeline|PostProcessTimeline` :!via `PlayFromStart`)
    (:`Update`
      (set `CameraComponent.PostProcessSettings` (make `PostProcessSettings` :`VignetteIntensity` _vignetteintensity :`DepthOfFieldFocalDistance` 1.0 :`DepthOfFieldScale` _scale) (`self.FirstPersonCamera`)))))

(event `InputAction|Pause` :paused true
  (params (Key :type "Key Structure" :default "AnyKey"))
  (:`Pressed`
    (for _array_element (`self.LevelSequences`)
      (if (`LevelSequencePlayer.IsPlaying` _array_element)
        (set `self.bCanPause` false)
        (break)
        (else
          (set `self.bCanPause` true))))
    (if (`self.bCanPause`)
      (if (`self.bPaused`)
        (set `self.bPaused` false)
        (bind _asndgamemode_bp (cast `/Game/Blueprints/NDGamemode_BP` (`GameplayStatics.GetGameMode`)))
        (bind _voice (`/Game/Blueprints/NDGamemode_BP.Voice` _asndgamemode_bp))
        (if (`/Game/Blueprints/Voice.bPaused` _voice)
          (`AudioComponent.SetPaused` (`/Game/Blueprints/Voice.Audio` _voice) false)
          (set `/Game/Blueprints/Voice.bPaused` false _voice))
        (`/Game/UI/PlayerHUD.SetPauseUI` (`/Game/Blueprints/NDGamemode_BP.WidgetReference` _asndgamemode_bp) false)
        (`GameplayStatics.SetGamePaused` false)
        (else
          (set `self.bPaused` true)
          (bind _asndgamemode_bp_2 (cast `/Game/Blueprints/NDGamemode_BP` (`GameplayStatics.GetGameMode`)))
          (bind _voice_2 (`/Game/Blueprints/NDGamemode_BP.Voice` _asndgamemode_bp_2))
          (bind _audio (`/Game/Blueprints/Voice.Audio` _voice_2))
          (if (`AudioComponent.IsPlaying` _audio)
            (`AudioComponent.SetPaused` _audio true)
            (set `/Game/Blueprints/Voice.bPaused` true _voice_2))
          (`/Game/UI/PlayerHUD.SetPauseUI` (`/Game/Blueprints/NDGamemode_BP.WidgetReference` _asndgamemode_bp_2) true)
          (`GameplayStatics.SetGamePaused` true)))
      (else
        (bind _asndgamemode_bp_3 (cast `/Game/Blueprints/NDGamemode_BP` (`GameplayStatics.GetGameMode`)))
        (`/Game/UI/PlayerHUD.PlayPauseAnimation` (`/Game/Blueprints/NDGamemode_BP.WidgetReference` _asndgamemode_bp_3))))))

(event `InputAction|Quit` :paused true
  (params (Key :type "Key Structure" :default "AnyKey"))
  (:`Pressed`
    (if (`self.bPaused`)
      (`KismetSystemLibrary.QuitGame` null "Quit"))))

(fn `ActivateShotParticle`
  (params (bCanShoot :type Boolean) (Cooldown :type "Float (double-precision)"))
  (if (not bCanShoot)
    (`ActorComponent.Activate` (`self.fx`) true))
  (return))

(fn `DamageEffects`
  (params (Health :type "Float (double-precision)"))
  (`|ExecutionSequence`
    (:`then_0`
      (`/Engine/EditorBlueprintResources/StandardMacros.DoOnce` false
        (:`Completed`
          (bind _asndgamemode_bp (cast `/Game/Blueprints/NDGamemode_BP` (`GameplayStatics.GetGameMode`)))
          (add `/Game/UI/PlayerHUD.OnRespawnFadeOut` (`/Game/Blueprints/NDGamemode_BP.WidgetReference` _asndgamemode_bp) (`|CreateDelegate` :!event `Respawn`)))))
    (:`then_1`
      (if (> (`self.Health`) 0.0)
        (set `CameraComponent.PostProcessSettings` (`self.CameraPostProcessing`) (`self.FirstPersonCamera`))
        (`self.UpdatePostProcessing`)
        (`GameplayStatics.PlayWorldCameraShake` "/Game/Blueprints/NDCameraShake.NDCameraShake_C" (`self.K2_GetActorLocation`) 0.0 500.0)
        (`KismetSystemLibrary.PrintString` "FX")))))

(fn `DeathCheck`
  (params (tmp :type "Float (double-precision)"))
  (`/Engine/EditorBlueprintResources/StandardMacros.CompareFloat` (`self.Health`)
    (:`==`
      _)
    (:`<`
      _))
  (bind _asndgamemode_bp (cast `/Game/Blueprints/NDGamemode_BP` (`GameplayStatics.GetGameMode`)))
  (bind _returnvalue (`EscapeGameModeBase.GetQuestStage` _asndgamemode_bp))
  (if (`|EnumInequality` _returnvalue "Die")
    (`self.DisableInput` null)
    (bind _widgetreference (`/Game/Blueprints/NDGamemode_BP.WidgetReference` _asndgamemode_bp))
    (`/Game/UI/PlayerHUD.FadeOutAndIn` _widgetreference 5.0)
    (else
      (`self.DisableInput` null)
      (`/Game/UI/PlayerHUD.FadeOutAndIn` _widgetreference 100.0))))

(fn `PlayChargeAudio`
  (params (ChargeTime :type "Float (double-precision)"))
  (bind _weaponaudio (`self.WeaponAudio`))
  (bind _weaponaudio_2 (`self.WeaponAudio`))
  ;[1 1 1] make sure we have some charge before we start
  (if (> ChargeTime 0.0)
    ;[1 1 1] Are we past the high shot threshhold? this determines what sound we will look at
    (if (>= ChargeTime 1.0)
      ;[1 1 1] If we are past the threshhold, have we set the nex max charge loop sound? If not then do it. If so, don't worry about it.
      (if (== (`AudioComponent.Sound` (`self.WeaponAudio`)) "/Game/Audio/weaponstart.weaponstart")
        (`AudioComponent.SetSound` _weaponaudio_2 "/Game/Audio/weaponloop.weaponloop")
        (`AudioComponent.Play` _weaponaudio_2 0.0))
      (else
        ;[1 1 1] If we have already set and played the sound, don't do it again. If not we are starting to charge so play the start sound.
        (if (not (== (`AudioComponent.Sound` (`self.WeaponAudio`)) "/Game/Audio/weaponstart.weaponstart"))
          (`AudioComponent.SetSound` _weaponaudio "/Game/Audio/weaponstart.weaponstart")
          (`AudioComponent.Play` _weaponaudio 0.0))))
    (return)
    (else
      (return))))

(fn `PlayFireAudio`
  (params (bCanShoot :type Boolean) (Cooldown :type "Float (double-precision)"))
  (bind _weaponaudio (`self.WeaponAudio`))
  (if (not bCanShoot)
    (`AudioComponent.SetSound` _weaponaudio "/Game/Audio/lasershot.lasershot")
    (`AudioComponent.Play` _weaponaudio 0.0)))

(fn `Respawn`
  (bind _asndgamemode_bp (cast `/Game/Blueprints/NDGamemode_BP` (`GameplayStatics.GetGameMode`))
    (:`then`
      (bind _returnvalue (`EscapeGameModeBase.GetQuestStage` _asndgamemode_bp))
      (if (`|EnumInequality` _returnvalue "Die")
        (set `self.Health` 100.0)
        (`/Game/UI/PlayerHUD.LerpHealth` (`/Game/Blueprints/NDGamemode_BP.WidgetReference` _asndgamemode_bp) (`self.Health`))
        (`self.K2_SetActorLocation` (`self.K2_GetActorLocation` (`self.RespawnPoint`)))
        (`self.EnableInput` null)
        (return)
        (else
          (`GameplayStatics.OpenLevel` "Credits")
          (return))))
    (:`CastFailed`
      (return))))

(fn `SetGunGlowBrightness`
  (params (ChargeTime :type "Float (double-precision)"))
  (`MaterialInstanceDynamic.SetScalarParameterValue` (`self.GunGlowMaterial`) "Brightness" (+ (* ChargeTime 5.0) 2.0))
  (set `/Game/Models/Weapon/Gun_AnimBP.Charge` ChargeTime (`self.AnimBP`)))

(fn `SetGunGlowColor`
  (params (bCanShoot :type Boolean) (Cooldown :type "Float (double-precision)"))
  (bind _animbp (`self.AnimBP`))
  (if (not bCanShoot)
    (`self.SetColorBlue` Cooldown)
    (`MaterialInstanceDynamic.SetScalarParameterValue` (`self.GunGlowMaterial`) "Brightness" 2.0)
    (set `/Game/Models/Weapon/Gun_AnimBP.bFired` true _animbp)
    (set `/Game/Models/Weapon/Gun_AnimBP.Charge` 0.0 _animbp)))

(fn `UserConstructionScript`
  (bind _returnvalue (`PrimitiveComponent.CreateDynamicMaterialInstance` (`self.Gun`) 1 null))
  (set `self.GunGlowMaterial` _returnvalue)
  (add `self.OnChargeShot` (`|CreateDelegate` :!event `SetGunGlowBrightness`))
  (add `self.OnChargeShot` (`|CreateDelegate` :!event `PlayChargeAudio`))
  (add `self.OnShoot` (`|CreateDelegate` :!event `SetGunGlowColor`))
  (add `self.OnShoot` (`|CreateDelegate` :!event `PlayFireAudio`))
  (add `self.OnShoot` (`|CreateDelegate` :!event `ActivateShotParticle`))
  (`ParticleSystemComponent.SetVectorParameter` (`self.fx`) "color" (`KismetMathLibrary.Conv_LinearColorToVector` (`KismetMathLibrary.MakeColor` 0.0 0.794 1.0)))
  (add `self.OnDamaged` (`|CreateDelegate` :!event `DeathCheck`))
  (set `self.BeginingGunLocation` (`SceneComponent.RelativeLocation` (`self.Gun`)))
  (add `self.OnSprint` (`|CreateDelegate` :!event `OnSprintEvent`)))