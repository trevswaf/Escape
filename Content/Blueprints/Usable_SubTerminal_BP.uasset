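; Usable submarine or sub-system terminal that can overheat and be cooled down when the player uses it.
; Overheat sets a flag and starts the smoke effect and audio.
; Tick shows a "Cooldown" prompt while the flag is set and clears it otherwise.
; Use resets the flag and stops both smoke and audio.
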(event `self.ReceiveTick`
  (params (DeltaSeconds :type "Float (single-precision)"))
  (if (`self.bIsOverheating`)
    (set `self.Prompt` "Cooldown")
    (else
      (set `self.Prompt` ""))))

(event `self.Use`
  (set `self.bIsOverheating` false)
  (`ActorComponent.Deactivate` (`self.Smoke`))
  (`AudioComponent.Stop` (`self.Audio`)))

(fn `Overheat`
  (set `self.bIsOverheating` true)
  (`ActorComponent.Activate` (`self.Smoke`) true)
  (`AudioComponent.Play` (`self.Audio`) 0.0))

(fn `UserConstructionScript`
  (`parent.UserConstructionScript`))