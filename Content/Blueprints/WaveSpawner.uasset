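; Wave spawner that starts repeating android waves when the game mode's quest stage changes to Die.
; On a looping timer, it asks each linked android spawner for one android while the live count is below a threshold.
; It overrides each new android's health and movement speeds and binds its death event, presumably to the function that decrements the count.
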(event `self.ReceiveBeginPlay`
  (bind _asndgamemode_bp (cast `/Game/Blueprints/NDGamemode_BP` (`GameplayStatics.GetGameMode`)))
  (add `EscapeGameModeBase.OnQuestStageSet` _asndgamemode_bp (delegate `StartSpawnLoop`)))

(event `StartSpawnLoop`
  (params (Stage :type "EQuestStage Enum"))
  (if (`|EnumEquality` Stage "Die")
    (`self.StartLoopWaveSpawn`)))

(fn `DecrementAndroidCount`
  (`/Engine/EditorBlueprintResources/StandardMacros.DecrementInt` (`self.CurrentAndroidCount`)
    (:`  `
      (return))))

(fn `SpawnWave`
  (for _array_element (`self.AndroidSpawners`)
    (if (< (`self.CurrentAndroidCount`) (`self.AndroidThreshhold`))
      (bind _androids (`/Game/Blueprints/AndroidSpawner.SpawnAndroid` _array_element 1))
      (`/Engine/EditorBlueprintResources/StandardMacros.IncrementInt` (`self.CurrentAndroidCount`)
        (:`  `
          (for _array_element_2 _androids
            (set `AndroidCharacter.Health` 150.0 _array_element_2)
            (set `AndroidCharacter.WalkSpeed` 500.0 _array_element_2)
            (set `AndroidCharacter.RunSpeed` 500.0 _array_element_2)
            (add `AndroidCharacter.OnDeath` _array_element_2 (`|CreateDelegate` :!event `DecrementAndroidCount`)))))))
  (return))

(fn `StartLoopWaveSpawn`
  (`self.SpawnWave`)
  (`KismetSystemLibrary.K2_SetTimerDelegate` (`|CreateDelegate` :!event `SpawnWave`) 10.0 true)
  (return))

(fn `UserConstructionScript`)