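; Enemy android character that melees the player and alerts other androids on sighting a pawn.
; Tick triggers the AnimBP attack when the player is near, then during damage frames halts movement and sphere-traces both hands to damage the player.
; Pawn sensing sets every android's DefaultLocation to the player.
; AnimBP and health events are bound, alongside functions for speed reset, footstep audio, hit explosions and death cleanup.
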(event `self.ReceiveBeginPlay`
  (bind _asandroid_anim_bp (cast `/Game/Character/AndroidAnimBP` (`SkeletalMeshComponent.GetAnimInstance` (`self.Mesh`))))
  (add `/Game/Character/AndroidAnimBP.OnAttackEnd` _asandroid_anim_bp (`|CreateDelegate` :!event `Reset Damage`))
  (add `/Game/Character/AndroidAnimBP.OnFootstep` _asandroid_anim_bp (`|CreateDelegate` :!event `PlayFootStep`)))

(event `self.ReceiveTick`
  (params (DeltaSeconds :type "Float (single-precision)"))
  (bind _returnvalue (`SceneComponent.GetSocketLocation` (`self.Mesh`) "RightHand"))
  (bind _returnvalue_2 (`SceneComponent.GetSocketLocation` (`self.Mesh`) "LeftHand"))
  (bind _asandroid_anim_bp (cast `/Game/Character/AndroidAnimBP` (`SkeletalMeshComponent.GetAnimInstance` (`self.Mesh`))))
  (if (and (`self.bCanDamage`) (<= (`self.GetDistanceTo` (`GameplayStatics.GetPlayerCharacter` 0)) 250.0) (> (`self.Health`) 0.0))
    (set `/Game/Character/AndroidAnimBP.bIsAttacking` true _asandroid_anim_bp)
    (if (`/Game/Character/AndroidAnimBP.bIsDamaging` _asandroid_anim_bp)
      (`|ExecutionSequence`
        (:`then_0`
          (set `self.RunSpeed` 0.0)
          (set `self.WalkSpeed` 0.0)
          (set `CharacterMovementComponent.MaxWalkSpeed` 0.0 (`self.CharacterMovement`)))
        (:`then_1`
          (bind _outhit (`KismetSystemLibrary.SphereTraceSingleForObjects` :`Start` _returnvalue :`End` _returnvalue :`Radius` 56.0 :`ObjectTypes` (`|MakeArray` "ObjectTypeQuery3" :!type "EObjectTypeQuery Enum") :`DrawDebugType` "ForOneFrame"))
          (bind _asfpscharacter_bp (cast `/Game/Blueprints/FPSCharacter_BP` (`.HitActor` (`GameplayStatics.BreakHitResult` _outhit))))
          (`self.OnDamageOverlap` null _asfpscharacter_bp null 0 false _outhit))
        (:`then_2`
          (bind _outhit_2 (`KismetSystemLibrary.SphereTraceSingleForObjects` :`Start` _returnvalue_2 :`End` _returnvalue_2 :`Radius` 56.0 :`ObjectTypes` (`|MakeArray` "ObjectTypeQuery3" :!type "EObjectTypeQuery Enum") :`DrawDebugType` "ForOneFrame"))
          (bind _asfpscharacter_bp_2 (cast `/Game/Blueprints/FPSCharacter_BP` (`.HitActor` (`GameplayStatics.BreakHitResult` _outhit_2))))
          (`self.OnDamageOverlap` null _asfpscharacter_bp_2 null 0 false _outhit_2))))))

(event `self.PawnSensingComponent.OnSeePawn`
  (params (Pawn :type "Pawn Object Reference"))
  (`self.AlertAndroidsOfPlayerPosition`))

(fn `AlertAndroidsOfPlayerPosition`
  (bind _outactors (`GameplayStatics.GetAllActorsOfClass` "AndroidCharacter_BP_C"))
  (for _array_element _outactors
    (set `AndroidCharacter.DefaultLocation` (`GameplayStatics.GetPlayerCharacter` 0) _array_element)
    (`self.InitDefaultLocation`))
  (return))

(fn `DamageEffects`
  (`GameplayStatics.SpawnEmitterAtLocation` "/Game/StarterContent/Particles/P_Explosion.P_Explosion" (`self.K2_GetActorLocation`) (`self.K2_GetActorRotation`))
  (bind _asandroid_anim_bp (cast `/Game/Character/AndroidAnimBP` (`SkeletalMeshComponent.GetAnimInstance` (`self.Mesh`)))
    (:`then`
      (set `/Game/Character/AndroidAnimBP.bIsDamaged` true _asandroid_anim_bp))
    (:`CastFailed`
      (`KismetSystemLibrary.PrintString` "u ufkced up")))
  (return))

(fn `DeathEffects`
  (`PrimitiveComponent.SetCollisionEnabled` (`self.CapsuleComponent`) "NoCollision")
  (`PrimitiveComponent.SetCollisionEnabled` (`self.Mesh`) "NoCollision")
  (`self.SetLifeSpan` 4.0)
  (return))

(fn `PlayFootStep`
  (`AudioComponent.Play` (`self.Audio`) 0.0))

(fn `Reset Damage`
  (set `self.bCanDamage` true)
  (set `self.RunSpeed` 500.0)
  (bind _output_get (set `self.WalkSpeed` 300.0))
  (set `CharacterMovementComponent.MaxWalkSpeed` _output_get (`self.CharacterMovement`)))

(fn `UserConstructionScript`
  (add `self.OnTakeDamage` (`|CreateDelegate` :!event `DamageEffects`))
  (add `self.OnDeath` (`|CreateDelegate` :!event `DeathEffects`)))